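; BP_Bones is an actor that drives a poseable skeletal mesh from Kinect body tracking.
; On BeginPlay it gets the first sensor from the KinectManager and initializes it, then closes it on EndPlay.
; Each tick it updates the skeleton and applies the first tracked skeleton's absolute joint rotations, combined with a fixed rotation offset, to bones matched by index in a name array, in world space.
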(event `self.ReceiveBeginPlay`
  ;[1 1 1] ini
  (bind _returnvalue (`KinectManager.GetSensor` (`KinectBPFunctionLibrary.KinectManager`)))
  (bind _output_get (set `self.kinect1` (`|GetArrayItem` _returnvalue)))
  (`KinectSensor.InitializeSensor` _output_get "/Game/Kinect_Skel/NewMaterial.NewMaterial"))

(event `self.ReceiveTick`
  (params (DeltaSeconds :type "Float (single-precision)"))
  (bind _kinect1 (`self.kinect1`))
  ;[1 1 1] Skeleton
  (`KinectSensor.UpdateSkeleton` _kinect1)
  ;[1 1 1] Rotate Bones
  (for (_array_element _array_index) (`.rotationAbsoluteQuaternion` (break `SkelStruct` (`|GetArrayItem` (`KinectSensor.FSkeletons` _kinect1))))
    (`PoseableMeshComponent.SetBoneRotationByName` (`self.PoseableMesh`) (`|GetArrayItem` (`self.boneNames`) _array_index) (`KismetMathLibrary.ComposeRotators` _array_element (struct :`Yaw` -90.0 :`Roll` 90.0)) "WorldSpace")))

(event `self.ReceiveEndPlay`
  (params (EndPlayReason :type "EEndPlayReason Enum" :default "Destroyed"))
  (`KinectSensor.CloseKinect` (`self.kinect1`)))

(fn `UserConstructionScript`)