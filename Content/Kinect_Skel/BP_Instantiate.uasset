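; Actor Blueprint that visualizes a Kinect-tracked skeleton as instanced static meshes, one per joint.
; BeginPlay initializes the first Kinect sensor with a material and spawns a row of twenty half-scale placeholder instances.
; Each Tick updates the skeleton and moves the instances to the first skeleton's joint positions, scaled up a hundredfold.
; EndPlay closes the Kinect.
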(event `self.ReceiveBeginPlay`
  ;[1 1 1] ini
  (bind _returnvalue (`KinectManager.GetSensor` (`KinectBPFunctionLibrary.KinectManager`)))
  (bind _output_get (set `self.kinect1` (`|GetArrayItem` _returnvalue)))
  (`KinectSensor.InitializeSensor` _output_get "/Game/Kinect_Skel/NewMaterial.NewMaterial")
  ;[1 1 1] ini instantiate
  (for _index (range 20)
    (`InstancedStaticMeshComponent.AddInstance` (`self.InstancedStaticMesh`) (`KismetMathLibrary.MakeTransform` (`KismetMathLibrary.MakeVector` (* _index 100.0)) (struct) (0.5 0.5 0.5)))))

(event `self.ReceiveTick`
  (params (DeltaSeconds :type "Float (single-precision)"))
  (bind _kinect1 (`self.kinect1`))
  ;[1 1 1] Skeleton
  (`KinectSensor.UpdateSkeleton` _kinect1)
  ;[1 1 1] update Instantiate Position
  (for (_array_element _array_index) (`.JointPosition` (break `SkelStruct` (`|GetArrayItem` (`KinectSensor.FSkeletons` _kinect1))))
    (`InstancedStaticMeshComponent.UpdateInstanceTransform` (`self.InstancedStaticMesh`) _array_index (`KismetMathLibrary.MakeTransform` (* _array_element 100.0) (struct) (0.5 0.5 0.5)) false true false)))

(event `self.ReceiveEndPlay`
  (params (EndPlayReason :type "EEndPlayReason Enum" :default "Destroyed"))
  (`KinectSensor.CloseKinect` (`self.kinect1`)))

(fn `UserConstructionScript`)